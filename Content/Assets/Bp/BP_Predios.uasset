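; BP_Predios is a building segment that requests a new building from the game mode as the player progresses.
; When BP_character overlaps its Colision component, it calls NovoPredio on BP_GM and destroys itself after a short delay.
; The Ponto function exposes world transforms from ArrowPredio and three ArrowBoost markers, apparently as placement points for the next building and boosts.
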(event `self.ReceiveBeginPlay`)

(event `self.Colision.OnComponentBeginOverlap`
  (params (OverlappedComponent :type "PrimitiveComponent Object Reference") (OtherActor :type "Actor Object Reference") (OtherComp :type "PrimitiveComponent Object Reference") (OtherBodyIndex :type Integer) (bFromSweep :type Boolean) (SweepResult :type "HitResult Structure (by ref)"))
  (cast `/Game/Assets/Bp/BP_character` OtherActor)
  (bind _asbp_gm (cast `/Game/Assets/Bp/BP_GM` (`GameplayStatics.GetGameMode`)))
  (`/Game/Assets/Bp/BP_GM.novoPredio` _asbp_gm)
  (`KismetSystemLibrary.Delay` 0.2)
  (`self.K2_DestroyActor`))

(fn `ponto`
  (returns (ponto :type "Transform Structure") (Pboost :type "Transform Structure") (Pboost2 :type "Transform Structure") (Pboost3 :type "Transform Structure"))
  (return (`SceneComponent.K2_GetComponentToWorld` (`self.ArrowPredio`)) (`SceneComponent.K2_GetComponentToWorld` (`self.ArrowBoost`)) (`SceneComponent.K2_GetComponentToWorld` (`self.ArrowBoost2`)) (`SceneComponent.K2_GetComponentToWorld` (`self.ArrowBoost3`))))

(fn `UserConstructionScript`)