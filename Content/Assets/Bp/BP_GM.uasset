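; BP_GM, apparently the game mode, builds a chained track of BP_Predios buildings with random birds and boost rings.
; BeginPlay spawns the initial run of buildings, each placed at the attach point returned by the previous one.
; NovoPredio appends one building, randomly spawning BP_Birds or BP_Boost_Ring at the stored Pbooster point.
; Some random branches then move Pbooster to one of the new building's three boost points for later spawns.
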(event `self.ReceiveBeginPlay`
  (for _ (range 61)
    (bind _returnvalue (`|SpawnActorFromClass` "/Game/Assets/Bp/BP_Predios.BP_Predios_C" (`self.netpoint`) "Undefined" "OverrideRootScale" null null))
    (bind _ponto (`/Game/Assets/Bp/BP_Predios.ponto` _returnvalue))
    (set `self.netpoint` _ponto)))

(fn `novoPredio`
  (bind _returnvalue (`KismetMathLibrary.RandomIntegerInRange` 0 10))
  (bind _returnvalue_2 (`KismetMathLibrary.RandomIntegerInRange` 0 10))
  (bind _returnvalue_3 (`|SpawnActorFromClass` "/Game/Assets/Bp/BP_Predios.BP_Predios_C" (`self.netpoint`) "Undefined" "OverrideRootScale" null null))
  (bind (_ponto _pboost _pboost2 _pboost3) (`/Game/Assets/Bp/BP_Predios.ponto` _returnvalue_3))
  (set `self.netpoint` _ponto)
  (if (== _returnvalue_2 1)
    (`|SpawnActorFromClass` "/Game/Assets/Blueprints/BP_Birds.BP_Birds_C" (`self.Pbooster`) "Undefined" "OverrideRootScale" null null)
    (if (== _returnvalue 1) :!label _label
      (set `self.Pbooster` _pboost)
      (elif (== _returnvalue 2)
        (set `self.Pbooster` _pboost2)
        (elif (== _returnvalue 0)
          (set `self.Pbooster` _pboost3))))
    (elif (== _returnvalue_2 2)
      (`|SpawnActorFromClass` "/Game/Assets/Bp/BP_Boost_Ring.BP_Boost_Ring_C" (`self.Pbooster`) "Undefined" "OverrideRootScale" null null)
      (goto _label)
      (elif (== _returnvalue_2 0)
        (goto _label)))))

(fn `UserConstructionScript`)